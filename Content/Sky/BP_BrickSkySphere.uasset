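; Sky sphere actor that runs an animated day/night and seasonal sky with sun, moon, stars and clouds.
; Construction creates dynamic instances for the sky material and the directional light's cloud light function.
; Each tick derives sun direction from latitude, axial tilt and date, plus a made-up moon path, then drives materials, fog and ambient tint through sun-height curves.
; One directional light switches between sun and moon; seasonal cloudiness shapes both cloud materials.
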(event EventTick
  (params (DeltaSeconds :type Float%20%28single-precision%29))
  (CallFunction|Update (Utilities|Time|GetGameTimeinSeconds)))

(fn ConstructionScript
  (bind _returnvalue (Math|Float|Loge 2.0))
  (bind _sky_sheet (Variables|Default|GetSky%20sheet))
  (bind _cloud_transmission (Variables|Clouds|GetCloud%20transmission))
  (bind _returnvalue_2 (Math|Float|Loge _cloud_transmission))
  (bind _returnvalue_3 (/ _returnvalue_2 2e+03))
  (bind _returnvalue_4 (/ _returnvalue_3 _returnvalue))
  ;[1 1 1] Create the sky material
  (bind _returnvalue_5 (Rendering|Material|CreateDynamicMaterialInstance (Variables|Default|GetSky%20Sphere%20mesh) 0 (Variables|Sky|GetSky%20material) :!class /Script/Engine.PrimitiveComponent))
  (Variables|Default|SetSky%20material%20instance _returnvalue_5)
  (Rendering|Material|SetScalarParameterValue (Variables|Default|GetSky%20material%20instance) "Cloud speed" (Variables|Clouds|GetCloud%20speed) :!class /Script/Engine.MaterialInstanceDynamic)
  (Rendering|Material|SetScalarParameterValue (Variables|Default|GetSky%20material%20instance) "Stars brightness" (Variables|Sky|GetStars%20brightness) :!class /Script/Engine.MaterialInstanceDynamic)
  (Rendering|Material|SetScalarParameterValue (Variables|Default|GetSky%20material%20instance) "Cloud altitude" (Variables|Clouds|GetCloud%20altitude) :!class /Script/Engine.MaterialInstanceDynamic)
  (Rendering|Material|SetScalarParameterValue (Variables|Default|GetSky%20material%20instance) "Cloud transmission" _returnvalue_4 :!class /Script/Engine.MaterialInstanceDynamic)
  ;[1 1 1] Setup sky sheet
  (Transformation|SetRelativeLocation _sky_sheet (Math|Vector|MakeVector 0.0 0.0 (Variables|Clouds|GetCloud%20altitude)) false)
  (Rendering|Material|SetMaterial _sky_sheet 0 (Variables|Default|GetSky%20material%20instance))
  ;[1 1 1] Create light function material instance
  (bind _returnvalue_6 (Rendering|Material|CreateDynamicMaterialInstance (Variables|Sky|GetLight%20function%20material) :!class /Script/Engine.KismetMaterialLibrary))
  (Variables|Default|SetLight%20function%20instance _returnvalue_6)
  (Rendering|Components|Light|SetLightFunctionMaterial (Variables|Default|GetDirectional%20Light) (Variables|Default|GetLight%20function%20instance))
  (Rendering|Material|SetScalarParameterValue (Variables|Default|GetLight%20function%20instance) "Cloud altitude" (Variables|Clouds|GetCloud%20altitude) :!class /Script/Engine.MaterialInstanceDynamic)
  (Rendering|Material|SetScalarParameterValue (Variables|Default|GetLight%20function%20instance) "Cloud transmission" _returnvalue_4 :!class /Script/Engine.MaterialInstanceDynamic)
  (CallFunction|Update 0.0))

(fn Update
  (params (TimeInSeconds :type Float%20%28single-precision%29))
  (bind _moon_color (Variables|Moon|GetMoon%20color))
  ;[1 1 1] Update sun direction
  (bind (_directiontosun _directiontomoon) (CallFunction|ComputeHeavenlyDirections TimeInSeconds))
  (CallFunction|UpdateMaterial (Class|KismetMathLibrary|MapRange (.Pitch (Class|KismetMathLibrary|BreakRot (Math|Rotator|MakeRotfromX (Math|Vector|NegateVector _directiontosun)))) -9e+01 9e+01 1.0 -1.0) _directiontosun _directiontomoon TimeInSeconds)
  ;[1 1 1] Update ambient lighting
  (Variables|/Script/Engine.PostProcessVolume|SetSettings (Variables|Sky|GetSky%20Ambient%20Post%20Process%20Volume) (Utilities|Struct|MakePostProcessSettings false false false false false false false false false false false false false false false true (.bOverride_AmbientCubemapIntensity (Utilities|Struct|BreakPostProcessSettings (Variables|/Script/Engine.PostProcessVolume|GetSettings (Variables|Sky|GetSky%20Ambient%20Post%20Process%20Volume)))) false false false false false false false false false false false false false false false false false false false false false false false false false false false false false false false false false false false false false false false false false false false false false false false false false false false false false false false false false false false false false false false false false false false false false false false false false false false false false false false false false false false "(R=1.000000,G=1.000000,B=1.000000,A=1.000000)" "(R=1.000000,G=1.000000,B=1.000000,A=1.000000)" 0.5 0.0 1.0 "(R=1.000000,G=0.000000,B=0.000000,A=1.000000)" "(R=0.000000,G=1.000000,B=0.000000,A=1.000000)" "(R=0.000000,G=0.000000,B=1.000000,A=1.000000)" 0.03 1.0 0.18 4.0 "(R=1.000000,G=1.000000,B=1.000000,A=1.000000)" 0.0 0.5 1.0 1.0 1.0 4.0 16.0 32.0 1e+02 "(R=0.500000,G=0.500000,B=0.500000,A=1.000000)" "(R=0.500000,G=0.500000,B=0.500000,A=1.000000)" "(R=0.500000,G=0.500000,B=0.500000,A=1.000000)" "(R=0.500000,G=0.500000,B=0.500000,A=1.000000)" "(R=0.500000,G=0.500000,B=0.500000,A=1.000000)" 1.0 "(R=0.500000,G=0.500000,B=0.500000,A=1.000000)" 0 1.0 0.0 0.64 5312.0 0.0 0.0 0.384 1.0 1.0 (Math|Curves|GetLinearColorValue (Variables|Sky|GetSky%20ambient%20tint%20by%20Sun%20Z) (Class|KismetMathLibrary|MapRange (.Pitch (Class|KismetMathLibrary|BreakRot (Math|Rotator|MakeRotfromX (Math|Vector|NegateVector _directiontosun)))) -9e+01 9e+01 1.0 -1.0)) (.AmbientCubemapIntensity (Utilities|Struct|BreakPostProcessSettings (Variables|/Script/Engine.PostProcessVolume|GetSettings (Variables|Sky|GetSky%20Ambient%20Post%20Process%20Volume)))) (.AmbientCubemap (Utilities|Struct|BreakPostProcessSettings (Variables|/Script/Engine.PostProcessVolume|GetSettings (Variables|Sky|GetSky%20Ambient%20Post%20Process%20Volume)))) 8e+01 98.300003 0.03 2.0 3.0 1.0 0.0 -8.0 4.0 1.0 "(R=1.000000,G=1.000000,B=1.000000,A=1.000000)" 3.0 8.0 0 "(R=1.000000,G=0.800000,B=0.400000,A=0.600000)" 0.0 "(R=0.000000,G=0.000000,B=0.000000,A=1.000000)" 0.0 0.0 0.5 1.0 4e+01 false 8e+03 5e+03 8e+02 2.0 3.0 5e+01 0.6 1.7 0.01 "(R=1.000000,G=1.000000,B=1.000000,A=1.000000)" 1.0 1.0 0 "DOFM_BokehDOF" 1e+03 0.0 3e+02 5e+02 0.0 15.0 15.0 15.0 0 0.4 1.0 0.08 0.0 0.5 5.0 0.5 1e+02 "AAM_TemporalAA" 1e+02 5e+01 0.6 (Utilities|Array|MakeArray)))
  ;[1 1 1] Set fog inscattering color
  (Class|ExponentialHeightFogComponent|SetFogInscatteringColor (Variables|Default|GetFog) (Math|Curves|GetLinearColorValue (Variables|Sky|GetHorizon%20color%20curve) (Class|KismetMathLibrary|MapRange (.Pitch (Class|KismetMathLibrary|BreakRot (Math|Rotator|MakeRotfromX (Math|Vector|NegateVector _directiontosun)))) -9e+01 9e+01 1.0 -1.0)))
  (Math|Float|CompareFloat (Class|KismetMathLibrary|MapRange (Class|KismetMathLibrary|MapRange (.Pitch (Class|KismetMathLibrary|BreakRot (Math|Rotator|MakeRotfromX (Math|Vector|NegateVector _directiontosun)))) -9e+01 9e+01 1.0 -1.0) 0.1 1.0 0.0 1.0) 0.0
    (:>
      ;[1 1 1] Update the directional light as the sun
      (Class|ExponentialHeightFogComponent|SetDirectionalInscatteringColor (Variables|Default|GetFog) (Math|Curves|GetLinearColorValue (Variables|Sun|GetSun%20color%20by%20sun%20Z) (Class|KismetMathLibrary|MapRange (.Pitch (Class|KismetMathLibrary|BreakRot (Math|Rotator|MakeRotfromX (Math|Vector|NegateVector _directiontosun)))) -9e+01 9e+01 1.0 -1.0)) :!label _label)
      (CallFunction|UpdateDirectionalLight (Math|Curves|GetLinearColorValue (Variables|Sun|GetSun%20color%20by%20sun%20Z) (Class|KismetMathLibrary|MapRange (.Pitch (Class|KismetMathLibrary|BreakRot (Math|Rotator|MakeRotfromX (Math|Vector|NegateVector _directiontosun)))) -9e+01 9e+01 1.0 -1.0)) (* (Variables|Sun|GetSun%20brightness) (Math|Float|Clamp(Float) (Class|KismetMathLibrary|MapRange (Class|KismetMathLibrary|MapRange (.Pitch (Class|KismetMathLibrary|BreakRot (Math|Rotator|MakeRotfromX (Math|Vector|NegateVector _directiontosun)))) -9e+01 9e+01 1.0 -1.0) 0.1 1.0 0.0 1.0) 0.0)) (Variables|Default|GetDirectional%20Light) _directiontosun))
    (:==
      (goto _label))
    (:<
      ;[1 1 1] Update the directional light as the moon
      (Class|ExponentialHeightFogComponent|SetDirectionalInscatteringColor (Variables|Default|GetFog) _moon_color)
      (CallFunction|UpdateDirectionalLight _moon_color (CallFunction|GetMoonBrightness _directiontomoon _directiontosun (- 0.0 (Class|KismetMathLibrary|MapRange (Class|KismetMathLibrary|MapRange (.Pitch (Class|KismetMathLibrary|BreakRot (Math|Rotator|MakeRotfromX (Math|Vector|NegateVector _directiontosun)))) -9e+01 9e+01 1.0 -1.0) 0.1 1.0 0.0 1.0))) (Variables|Default|GetDirectional%20Light) _directiontomoon)))
  (Math|Float|CompareFloat (Class|KismetMathLibrary|MapRange (Class|KismetMathLibrary|MapRange (.Pitch (Class|KismetMathLibrary|BreakRot (Math|Rotator|MakeRotfromX (Math|Vector|NegateVector _directiontosun)))) -9e+01 9e+01 1.0 -1.0) -0.25 1.0 0.0 1.0) 0.0
    (:>
      (CallFunction|UpdateCloudLighting _directiontosun (* (Variables|Sun|GetSun%20brightness) (* (Math|Float|Clamp(Float) (Class|KismetMathLibrary|MapRange (Class|KismetMathLibrary|MapRange (.Pitch (Class|KismetMathLibrary|BreakRot (Math|Rotator|MakeRotfromX (Math|Vector|NegateVector _directiontosun)))) -9e+01 9e+01 1.0 -1.0) -0.25 1.0 0.0 1.0) 0.0) (Math|Float|Clamp(Float) (Class|KismetMathLibrary|MapRange (Class|KismetMathLibrary|MapRange (.Pitch (Class|KismetMathLibrary|BreakRot (Math|Rotator|MakeRotfromX (Math|Vector|NegateVector _directiontosun)))) -9e+01 9e+01 1.0 -1.0) -0.25 1.0 0.0 1.0) 0.0))) (Math|Curves|GetLinearColorValue (Variables|Sun|GetSun%20color%20by%20sun%20Z) (Class|KismetMathLibrary|MapRange (.Pitch (Class|KismetMathLibrary|BreakRot (Math|Rotator|MakeRotfromX (Math|Vector|NegateVector _directiontosun)))) -9e+01 9e+01 1.0 -1.0))))
    (:==
      (CallFunction|UpdateCloudLighting _directiontomoon (CallFunction|GetMoonBrightness _directiontomoon _directiontosun (- 0.0 (Class|KismetMathLibrary|MapRange (Class|KismetMathLibrary|MapRange (.Pitch (Class|KismetMathLibrary|BreakRot (Math|Rotator|MakeRotfromX (Math|Vector|NegateVector _directiontosun)))) -9e+01 9e+01 1.0 -1.0) -0.25 1.0 0.0 1.0))) (Variables|Moon|GetMoon%20color) :!label _label_2))
    (:<
      (goto _label_2)))
  (CallFunction|UpdateDirectionalLight (Math|Curves|GetLinearColorValue (Variables|Sun|GetSun%20color%20by%20sun%20Z) (Class|KismetMathLibrary|MapRange (.Pitch (Class|KismetMathLibrary|BreakRot (Math|Rotator|MakeRotfromX (Math|Vector|NegateVector _directiontosun)))) -9e+01 9e+01 1.0 -1.0)) 0.0 (Variables|Default|GetSun%20light%20shafts) _directiontosun))

(fn ComputeHeavenlyDirections
  (params (TimeInSeconds :type Float%20%28single-precision%29))
  (bind _startday (Variables|Time|GetStartDay))
  (bind _secondsperday (Variables|Time|GetSecondsPerDay))
  (bind _returnvalue (/ TimeInSeconds _secondsperday))
  (bind _returnvalue_2 (+ _startday _returnvalue))
  (return (Math|Vector|UnrotateVector (Math|Vector|RotateVector "1.000000, 0, 0" (Class|KismetMathLibrary|MakeRot 0.0 (* (/ (+ (Variables|Time|GetStartDay) (/ TimeInSeconds (Variables|Time|GetSecondsPerDay))) (Variables|Time|GetDaysPerYear)) 3.6e+02) 0.0)) (Math|Rotator|CombineRotators (Class|KismetMathLibrary|MakeRot (- 9e+01 (Variables|Sun|GetLatitude)) 0.0 0.0) (Math|Rotator|CombineRotators (Class|KismetMathLibrary|MakeRot 0.0 (* (+ (/ TimeInSeconds (Variables|Time|GetSecondsPerDay)) (Variables|Time|GetStartDay)) -3.6e+02) 0.0) (Class|KismetMathLibrary|MakeRot (Variables|Sun|GetEclipticTilt) 0.0 0.0)))) (Math|Rotator|GetRotationXVector (Class|KismetMathLibrary|MakeRot (+ (* (Math|Trig|Cos(Degrees) (* _returnvalue_2 3.6e+02)) (Variables|Moon|GetMoon%20Angle%20Variance)) (Variables|Moon|GetMoon%20Angle%20Median)) (+ (* _returnvalue_2 3.6e+02) 1.5e+02) 0.0))))

(fn UpdateDirectionalLight
  (params (Color :type Linear%20Color%20Structure) (Brightness :type Float%20%28single-precision%29) (Light%20Component :type Directional%20Light%20Component%20Object%20Reference) (Direction%20to%20light :type Vector))
  (Transformation|SetWorldRotation Light%20Component (Math|Rotator|MakeRotfromX (Math|Vector|NegateVector Direction%20to%20light)) false)
  (Rendering|Components|Light|SetLightColor Light%20Component Color)
  (Class|LightComponent|SetBrightness Light%20Component Brightness))

(fn UpdateMaterial
  (params (Sun%20height :type Float%20%28single-precision%29) (Direction%20to%20sun :type Vector) (Direction%20to%20moon :type Vector) (Time%20in%20seconds :type Float%20%28single-precision%29))
  (bind _returnvalue (Math|Float|Absolute(Float) Sun%20height))
  (bind _returnvalue_2 (Utilities|Time|GetGameTimeinSeconds))
  (bind _returnvalue_3 (Math|Float|Loge 2.0))
  (bind _secondsperday (Variables|Time|GetSecondsPerDay))
  (bind _startday (Variables|Time|GetStartDay))
  (bind _sky_material_instance (Variables|Default|GetSky%20material%20instance))
  (bind _cloud_speed (Variables|Clouds|GetCloud%20speed))
  (bind _light_function_instance (Variables|Default|GetLight%20function%20instance))
  (bind _cloud_thickness (Variables|Clouds|GetCloud%20thickness))
  (bind _cloudiness_by_season (Variables|Clouds|GetCloudiness%20by%20season))
  (bind _cloud_transmission (Variables|Clouds|GetCloud%20transmission))
  (bind _daysperyear (Variables|Time|GetDaysPerYear))
  (bind _returnvalue_4 (/ Time%20in%20seconds _secondsperday))
  (bind _returnvalue_5 (* _returnvalue_2 _cloud_speed))
  (bind _returnvalue_6 (* "0.000000,-1.000000,0.200000" _returnvalue_5))
  (bind _returnvalue_7 (+ _returnvalue_4 _startday))
  (bind _returnvalue_8 (Math|Conversions|ToLinearColor(Vector) _returnvalue_6))
  (bind _returnvalue_9 (/ _returnvalue_7 _daysperyear))
  (bind _returnvalue_10 (Math|Float|Fraction _returnvalue_9))
  (bind _returnvalue_11 (Math|Curves|GetFloatValue _cloudiness_by_season _returnvalue_10))
  (bind _returnvalue_12 (Math|Float|Clamp(Float) _returnvalue_11 0.001 0.999))
  (bind _returnvalue_13 (/ 1.0 _returnvalue_12))
  (bind _returnvalue_14 (Math|Float|Lerp 0.75 _cloud_transmission _returnvalue_12))
  (bind _returnvalue_15 (* _returnvalue_12 _cloud_thickness))
  (bind _returnvalue_16 (- 0.0 _returnvalue_13))
  (bind _returnvalue_17 (/ _returnvalue_15 5e+02))
  (bind _returnvalue_18 (Math|Float|Loge _returnvalue_14))
  (bind _returnvalue_19 (/ _returnvalue_18 1e+03))
  (bind _returnvalue_20 (+ _returnvalue_16 1.0))
  (bind _returnvalue_21 (/ _returnvalue_19 _returnvalue_3))
  (bind _linearcolor (Utilities|Struct|MakeLinearColor _returnvalue_13 _returnvalue_20 _returnvalue_17 _returnvalue_15))
  (Rendering|Material|SetVectorParameterValue _sky_material_instance "Sun direction" (Math|Conversions|ToLinearColor(Vector) Direction%20to%20sun) :!class /Script/Engine.MaterialInstanceDynamic)
  (Rendering|Material|SetVectorParameterValue _sky_material_instance "Moon direction" (Math|Conversions|ToLinearColor(Vector) Direction%20to%20moon) :!class /Script/Engine.MaterialInstanceDynamic)
  (Rendering|Material|SetVectorParameterValue _sky_material_instance "Sun color" (* (Math|Curves|GetLinearColorValue (Variables|Sun|GetSun%20color%20by%20sun%20Z) Sun%20height) (Variables|Sun|GetSun%20brightness)) :!class /Script/Engine.MaterialInstanceDynamic)
  (Rendering|Material|SetVectorParameterValue _sky_material_instance "Moon color" (* (Variables|Moon|GetMoon%20color) (Variables|Moon|GetMoon%20brightness)) :!class /Script/Engine.MaterialInstanceDynamic)
  (Rendering|Material|SetVectorParameterValue _sky_material_instance "Horizon color" (Math|Curves|GetLinearColorValue (Variables|Sky|GetHorizon%20color%20curve) Sun%20height) :!class /Script/Engine.MaterialInstanceDynamic)
  (Rendering|Material|SetVectorParameterValue _sky_material_instance "Zenith color" (Math|Curves|GetLinearColorValue (Variables|Sky|GetZenith%20color%20curve) Sun%20height) :!class /Script/Engine.MaterialInstanceDynamic)
  (Rendering|Material|SetScalarParameterValue _sky_material_instance "Horizon falloff" (Math|Float|Lerp 3.0 8.0 _returnvalue) :!class /Script/Engine.MaterialInstanceDynamic)
  (Rendering|Material|SetScalarParameterValue _sky_material_instance "Sun height" _returnvalue :!class /Script/Engine.MaterialInstanceDynamic)
  (Rendering|Material|SetVectorParameterValue _sky_material_instance "Cloud pan" _returnvalue_8 :!class /Script/Engine.MaterialInstanceDynamic)
  (Rendering|Material|SetVectorParameterValue _sky_material_instance "Cloud noise parameters" _linearcolor :!class /Script/Engine.MaterialInstanceDynamic)
  (Rendering|Material|SetScalarParameterValue _sky_material_instance "Cloud transmission" _returnvalue_21 :!class /Script/Engine.MaterialInstanceDynamic)
  (Rendering|Material|SetVectorParameterValue _light_function_instance "Cloud noise parameters" _linearcolor :!class /Script/Engine.MaterialInstanceDynamic)
  (Rendering|Material|SetVectorParameterValue _light_function_instance "Cloud pan" _returnvalue_8 :!class /Script/Engine.MaterialInstanceDynamic)
  (Rendering|Material|SetScalarParameterValue _light_function_instance "Cloud transmission" _returnvalue_21 :!class /Script/Engine.MaterialInstanceDynamic))

(fn GetTimeinDays
  (return (+ (/ (Utilities|Time|GetGameTimeinSeconds) (Variables|Time|GetSecondsPerDay)) (Variables|Time|GetStartDay))))

(fn UpdateCloudLighting
  (params (Direction%20to%20light :type Vector) (Brightness :type Float%20%28single-precision%29) (Color :type Linear%20Color%20Structure))
  (bind (_x _y _z) (Math|Vector|BreakVector Direction%20to%20light))
  (bind _sky_material_instance (Variables|Default|GetSky%20material%20instance))
  (bind _returnvalue (Math|Float|Max(Float) _z 0.35))
  (bind _linearcolor (Utilities|Struct|MakeLinearColor _x _y _returnvalue 0.0))
  (Rendering|Material|SetVectorParameterValue (Variables|Default|GetLight%20function%20instance) "Light direction" _linearcolor :!class /Script/Engine.MaterialInstanceDynamic)
  (Rendering|Material|SetVectorParameterValue _sky_material_instance "Cloud light direction" _linearcolor :!class /Script/Engine.MaterialInstanceDynamic)
  (Rendering|Material|SetVectorParameterValue _sky_material_instance "Cloud light color" (* Color Brightness) :!class /Script/Engine.MaterialInstanceDynamic))

(fn GetMoonBrightness
  (params (Direction%20to%20moon :type Vector) (Direction%20to%20sun :type Vector) (Blend :type Float%20%28single-precision%29))
  (return (* (Variables|Moon|GetMoon%20brightness) (Math|Float|Clamp(Float) (* (Class|KismetMathLibrary|MapRange (Math|Vector|DotProduct (Math|Vector|NegateVector Direction%20to%20moon) Direction%20to%20sun) -1.0 1.0 0.0 1.0) Blend) 0.01))))