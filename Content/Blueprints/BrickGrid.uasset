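; Voxel-style brick terrain actor that hosts a BrickGrid, initialized from grid parameters in the construction script.
; Each tick it updates the grid around the camera position with draw and collision distance limits, generating terrain through an InitRegion callback under a per-frame region cap.
; New and loaded games run the same update with a very high cap to build surroundings at once; saving and loading copy the grid data.
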(event EventTick
  (params (DeltaSeconds :type Float%20%28single-precision%29))
  (Class|BrickGridComponent|Update (Variables|Default|GetBrickGrid) (Transformation|GetWorldLocation (Variables|/Script/Engine.PlayerCameraManager|GetTransformComponent (Game|GetPlayerCameraManager 0))) (Variables|BrickGrid|GetMaxDrawDistance) (Variables|BrickGrid|GetMaxCollisionDistance) (Variables|Default|GetMaxRegionsToCreatePerFrame) (EventDispatchers|CreateEvent self :!event InitRegion)))

(fn ConstructionScript
  (Class|BrickGridComponent|Init (Variables|Default|GetBrickGrid) (Variables|BrickGrid|GetGridParameters)))

(fn InitRegion
  (params (Coordinates :type Int%203%20Structure))
  (Class|BrickTerrainGenerationLibrary|InitRegion (Variables|BrickGrid|GetTerrainGenerationParameters) (Variables|Default|GetBrickGrid) Coordinates))

(fn LoadGame
  (params (SavedGame :type Brick%20Save%20Game%20Object%20Reference))
  (Class|BrickGridComponent|SetData (Variables|Default|GetBrickGrid) (Variables|/Game/Blueprints/BrickSaveGame.BrickSaveGame_C|GetBrickGridData SavedGame))
  (CallFunction|InitGridRenderingandCollision))

(fn SaveGame
  (params (SavedGame :type Brick%20Save%20Game%20Object%20Reference))
  (Variables|/Game/Blueprints/BrickSaveGame.BrickSaveGame_C|SetBrickGridData SavedGame (Class|BrickGridComponent|GetData (Variables|Default|GetBrickGrid))))

(fn NewGame
  (CallFunction|InitGridRenderingandCollision))

(fn InitGridRenderingandCollision
  (Class|BrickGridComponent|Update (Variables|Default|GetBrickGrid) (Transformation|GetWorldLocation (Variables|/Script/Engine.PlayerCameraManager|GetTransformComponent (Game|GetPlayerCameraManager 0))) (Variables|BrickGrid|GetMaxDrawDistance) (Variables|BrickGrid|GetMaxCollisionDistance) 100000 (EventDispatchers|CreateEvent self :!event InitRegion)))