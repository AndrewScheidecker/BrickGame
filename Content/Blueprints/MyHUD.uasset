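; MyHUD is a HUD Blueprint that shows the player which material is currently selected for placing.
; On each DrawHUD it casts the owning pawn to MyCharacter and uses that character's MaterialIndex to look up a name in MaterialNames.
; It draws the "placing:" label with that name in yellow text, positioned from screen-size fractions near the lower center.
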(event EventDrawHUD
  (params (SizeX :type Integer) (SizeY :type Integer))
  (bind _returnvalue (/ SizeX 10))
  (bind _returnvalue_2 (/ _returnvalue 2))
  (bind _asmycharacter_c (Utilities|Casting|CastToMyCharacter (Class|HUD|GetOwningPawn)))
  (HUD|DrawText (Utilities|String|Append "placing: " (Utilities|Array|Get(acopy) (Variables|Default|GetMaterialNames) (Variables|/Game/Blueprints/MyCharacter.MyCharacter_C|GetMaterialIndex _asmycharacter_c))) "(R=1.000000,G=0.828464,B=0.000000,A=1.000000)" (Math|Conversions|ToFloat(Integer) (- (/ SizeX 2) _returnvalue_2)) (Math|Conversions|ToFloat(Integer) (- (- SizeY (/ SizeY 5)) _returnvalue_2)) 0 1.0 false))

(fn ConstructionScript)