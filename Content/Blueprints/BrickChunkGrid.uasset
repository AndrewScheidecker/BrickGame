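; Brick chunk grid actor that generates a brick world in chunks around the player's camera through its ChunkGrid component.
; When a chunk initializes, it loops over the chunk's X and Y size and fills one layer with a single material, resetting the runaway-loop counter per brick.
; Every tick it passes the player camera manager's world location to the grid to update its camera position.
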(event OnInitChunk(ChunkGrid)
  (params (Coordinates :type Chunk%20Coordinates%20Structure%20%28by%20ref%29) (Chunk :type Brick%20Chunk%20Component%20Object%20Reference))
  (bind _chunkgrid (Variables|Default|GetChunkGrid))
  (bind _chunkparameters (Variables|/Script/BrickGrid.BrickChunkGridComponent|GetChunkParameters _chunkgrid))
  (bind (_sizex _sizey) (Utilities|Struct|BreakBrickChunkParameters _chunkparameters))
  (for _index (range 0 (- _sizex 1))
    (for _index_2 (range 0 (- _sizey 1))
      (Class|BrickChunkComponent|SetBrick Chunk _index _index_2 0 1)
      (Class|SuperLoopLibrary|ResetRunawayLoopCounter))))

(event EventTick
  (params (DeltaSeconds :type Float%20%28single-precision%29))
  (Class|BrickChunkGridComponent|UpdateCameraPosition (Variables|Default|GetChunkGrid) (Transformation|GetWorldLocation (Variables|/Script/Engine.PlayerCameraManager|GetTransformComponent (Game|GetPlayerCameraManager 0)))))

(fn ConstructionScript)