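; Game mode for a brick-grid game that saves and restores the world and player position through one "World" save slot.
; BeginPlay caches the level's BrickGrid, and PostLogin loads the slot into it and moves the joining player's pawn to the saved transform.
; The save command writes grid and player transform to the slot.
; The load command only calls Open Level, with no level name set, leaving restoration to PostLogin.
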(event OnCommand(LoadCommand)
  (Game|OpenLevel(byName) "None" false))

(event OnCommand(SaveCommand)
  (bind _returnvalue (SaveGame|CreateSaveGameObject "/Game/Blueprints/BrickSaveGame.BrickSaveGame_C"))
  (bind _asbricksavegame_c (Utilities|Casting|CastToBrickSaveGame _returnvalue))
  (Default|SaveGame (Variables|Default|GetBrickGrid) _asbricksavegame_c)
  (Variables|/Game/Blueprints/BrickSaveGame.BrickSaveGame_C|SetPlayerTransform _asbricksavegame_c (Transformation|GetActorTransform (Game|GetPlayerCharacter 0)))
  (SaveGame|SaveGametoSlot _asbricksavegame_c "World" (Class|KismetSystemLibrary|MakeLiteralInteger)))

(event EventBeginPlay
  (bind _outactors (Actor|GetAllActorsOfClass "/Game/Blueprints/BrickGrid.BrickGrid_C"))
  (bind _asbrickgrid_c (Utilities|Casting|CastToBrickGrid (Utilities|Array|Get(acopy) _outactors)))
  (Variables|Default|SetBrickGrid _asbrickgrid_c))

(event EventPostLogin
  (params (NewPlayer :type Player%20Controller%20Object%20Reference))
  (bind _returnvalue (SaveGame|LoadGamefromSlot "World" (Class|KismetSystemLibrary|MakeLiteralInteger)))
  (bind _asbricksavegame_c (Utilities|Casting|CastToBrickSaveGame _returnvalue))
  (Default|LoadGame (Variables|Default|GetBrickGrid) _asbricksavegame_c)
  (Transformation|SetActorTransform (Pawn|GetControlledPawn NewPlayer) (Variables|/Game/Blueprints/BrickSaveGame.BrickSaveGame_C|GetPlayerTransform _asbricksavegame_c)))

(fn ConstructionScript)