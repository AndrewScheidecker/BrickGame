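; Player character Blueprint for a voxel brick-building game, with brick placing and removal, mouse-wheel material selection and a flashlight toggle.
; Each tick, a line trace along the control rotation positions destroy and create preview boxes on the aimed BrickChunkComponent.
; Target cells come from nudging the hit point half a brick along either normal direction and flooring it in chunk space.
; Fire release places the selected material; right-mouse release clears the hit brick.
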(event EventTick
  (params (DeltaSeconds :type Float%20%28single-precision%29))
  (CallFunction|UpdatePreviewBricks))

(event Input|ActionEvents|InputActionFire
  (:Pressed
    (CallFunction|UpdatePreviewBricks))
  (:Released
    (CallFunction|CreateBrick)))

(event Input|ActionEvents|InputActionFlashlight
  (:Released
    (Variables|Default|SetFlashLightEnabled (not (Variables|Default|GetFlashLightEnabled)))
    (CallFunction|UpdateFlashlight)))

(event Input|MouseEvents|MouseWheelDown
  (bind _returnvalue (Class|KismetSystemLibrary|MakeLiteralInteger 8))
  (:Released
    (Variables|Default|SetMaterialIndex (Math|Integer|%(Integer) (+ (Variables|Default|GetMaterialIndex) (- _returnvalue 1)) _returnvalue))))

(event Input|MouseEvents|MouseWheelUp
  (:Released
    (Variables|Default|SetMaterialIndex (Math|Integer|%(Integer) (+ (Variables|Default|GetMaterialIndex) 1) (Class|KismetSystemLibrary|MakeLiteralInteger 8)))))

(event Input|MouseEvents|RightMouseButton
  (:Released
    (CallFunction|DestroyBrick)))

(fn ConstructionScript)

(fn UpdateFlashlight
  (bind _variable (|LocalVariable))
  (if (Variables|Default|GetFlashLightEnabled)
    (|Assign _variable (Variables|Default|GetFlashlightBrightness))
    (else
      (|Assign _variable 0.0)))
  (Class|LightComponent|SetBrightness (Variables|Default|GetFlashlight) _variable))

(fn UpdatePreviewBricks
  (bind _createpreviewbrick (Variables|Default|GetCreatePreviewBrick))
  (bind _destroypreviewbrick (Variables|Default|GetDestroyPreviewBrick))
  (bind _hit (CallFunction|TraceAim))
  (bind _asbrickchunkcomponent (Utilities|Casting|CastToBrickChunkComponent (.HitComponent (Collision|BreakHitResult _hit)))
    (:then
      (bind (_brickx _bricky _brickz) (CallFunction|GetAimedBrickCoordinates _asbrickchunkcomponent (.Location (Collision|BreakHitResult _hit)) (Math|Vector|NegateVector (.Normal (Collision|BreakHitResult _hit)))))
      (CallFunction|SetPreviewBrickTransform _asbrickchunkcomponent _brickx _bricky _brickz _destroypreviewbrick 1.0)
      (bind (_brickx_2 _bricky_2 _brickz_2) (CallFunction|GetAimedBrickCoordinates _asbrickchunkcomponent (.Location (Collision|BreakHitResult _hit)) (.Normal (Collision|BreakHitResult _hit))))
      (CallFunction|SetPreviewBrickTransform _asbrickchunkcomponent _brickx_2 _bricky_2 _brickz_2 _createpreviewbrick 0.6)
      (bind _asbrickchunkgridcomponent (Utilities|Casting|CastToBrickChunkGridComponent (Transformation|GetAttachParent _asbrickchunkcomponent))
        (:then
          (Utilities|IsValid (Utilities|Struct|BreakBrickMaterial (Utilities|Array|Get(acopy) (.Materials (Utilities|Struct|BreakBrickChunkParameters (Variables|/Script/BrickGrid.BrickChunkGridComponent|GetChunkParameters _asbrickchunkgridcomponent))) (Variables|Default|GetMaterialIndex)))
            (:Is%20Valid
              (Rendering|Material|SetMaterial _createpreviewbrick 0 (Utilities|Struct|BreakBrickMaterial (Utilities|Array|Get(acopy) (.Materials (Utilities|Struct|BreakBrickChunkParameters (Variables|/Script/BrickGrid.BrickChunkGridComponent|GetChunkParameters _asbrickchunkgridcomponent))) (Variables|Default|GetMaterialIndex)))))
            (:Is%20Not%20Valid
              (Development|SetHiddeninGame _createpreviewbrick true false :!label _label))))
        (:CastFailed
          _)))
    (:CastFailed
      (Development|SetHiddeninGame _destroypreviewbrick true false)
      (goto _label)))
  (return _asbrickchunkcomponent _brickx _bricky _brickz _brickx_2 _bricky_2 _brickz_2))

(fn CreateBrick
  (bind (_brickchunkcomponent _destroybrickx _destroybricky _destroybrickz _createbrickx _createbricky _createbrickz) (CallFunction|UpdatePreviewBricks))
  (Utilities|IsValid _brickchunkcomponent
    (:Is%20Valid
      (Class|BrickChunkComponent|SetBrick _brickchunkcomponent _createbrickx _createbricky _createbrickz (Variables|Default|GetMaterialIndex)))))

(fn TraceAim
  (bind _returnvalue (Transformation|GetActorLocation))
  (bind _returnvalue_2 (+ "0, 0,64.000000" _returnvalue))
  (bind _outhit (Collision|LineTraceByChannel _returnvalue_2 (+ _returnvalue_2 (* (Math|Vector|RotateVector "1.000000,0.000000, 0" (Pawn|GetControlRotation :!class /Script/Engine.Pawn)) (Variables|Default|GetAimRange))) "TraceTypeQuery1" false 0 "None"))
  (return _outhit))

(fn DestroyBrick
  (bind _hit (CallFunction|TraceAim))
  (bind _asbrickchunkcomponent (Utilities|Casting|CastToBrickChunkComponent (.HitComponent (Collision|BreakHitResult _hit))))
  (bind (_brickx _bricky _brickz) (CallFunction|GetAimedBrickCoordinates _asbrickchunkcomponent (.Location (Collision|BreakHitResult _hit)) (Math|Vector|NegateVector (.Normal (Collision|BreakHitResult _hit)))))
  (Class|BrickChunkComponent|SetBrick _asbrickchunkcomponent _brickx _bricky _brickz))

(fn GetAimedBrickCoordinates
  (params (BrickChunk :type Brick%20Chunk%20Component%20Object%20Reference) (SurfaceLocation :type Vector) (Normal :type Vector))
  (bind _returnvalue (Transformation|GetWorldScale BrickChunk))
  (bind _returnvalue_2 (Transformation|GetWorldTransform BrickChunk))
  (bind _returnvalue_3 (* Normal 0.5))
  (bind _returnvalue_4 (* _returnvalue_3 _returnvalue))
  (bind _returnvalue_5 (+ SurfaceLocation _returnvalue_4))
  (bind _returnvalue_6 (Math|Transform|InverseTransformLocation _returnvalue_2 _returnvalue_5))
  (bind (_x _y _z) (Math|Vector|BreakVector _returnvalue_6))
  (return (Math|Float|Floor _x) (Math|Float|Floor _y) (Math|Float|Floor _z)))

(fn SetPreviewBrickTransform
  (params (BrickChunk :type Brick%20Chunk%20Component%20Object%20Reference) (X :type Integer) (Y :type Integer) (Z :type Integer) (PreviewBox :type Primitive%20Component%20Object%20Reference) (ScaleFactor :type Float%20%28single-precision%29))
  (Transformation|SetWorldTransform PreviewBox (Math|Transform|ComposeTransforms (Math|Transform|MakeTransform (+ (Math|Vector|MakeVector (Math|Conversions|ToFloat(Integer) X) (Math|Conversions|ToFloat(Integer) Y) (Math|Conversions|ToFloat(Integer) Z)) "0.500000,0.500000,0.500000") "0, 0, 0" (Math|Conversions|ToVector(Float) ScaleFactor)) (Transformation|GetWorldTransform BrickChunk)) false)
  (Development|SetHiddeninGame PreviewBox false false))